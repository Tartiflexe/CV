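; Orbital beam effect actor that moves a static mesh out to a firing pose, plays a Niagara beam with camera shake, then returns it.
; An idle spin on Tick pauses through a Gate when FxActivation starts a timeline blending location, rotation and scale from the BeginPlay transform.
; A FlipFlop on timeline completion alternates between the delayed beam-and-reverse sequence and re-arming the DoOnce and spin.
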(event `self.ReceiveBeginPlay`
  (`parent.ReceiveBeginPlay`)
  (set `self.Transform_0` (`SceneComponent.K2_GetComponentToWorld` (`self.StaticMesh`))))

(event `self.ReceiveTick`
  (params (DeltaSeconds :type "Float (single-precision)"))
  (`parent.ReceiveTick` DeltaSeconds)
  (`/Engine/EditorBlueprintResources/StandardMacros.Gate` false :!label _label
    (:`Exit`
      (`self.K2_AddActorLocalRotation` (struct :`Yaw` 1.0))
      (`self.K2_AddActorWorldRotation` (struct :`Yaw` 1.0)))))

(event `/Game/Blueprints/cv_interface.Fx_Activation`
  (`/Engine/EditorBlueprintResources/StandardMacros.DoOnce` false :!label _label_2
    (:`Completed`
      (`|ExecutionSequence`
        (:`then_0`
          (goto _label :!via `Close`))
        (:`then_1`
          (bind (_direction _newtrack_0) (`Timeline|Timeline_0` :!via `PlayFromStart` :!label _label_3)
            (:`Update`
              (`SceneComponent.K2_SetWorldTransform` (`self.StaticMesh`) (`KismetMathLibrary.MakeTransform` (`KismetMathLibrary.VLerp` (.location (`self.Transform_0`)) (+ (.location (`self.Transform_0`)) (2000.0 8000.0 1500.0)) _newtrack_0) (`KismetMathLibrary.RLerp` (.rotation (`self.Transform_0`)) (`KismetMathLibrary.MakeRotator` (+ (.roll (.rotation (`self.Transform_0`))) 20.0) (.pitch (.rotation (`self.Transform_0`))) (+ (.yaw (.rotation (`self.Transform_0`))) 360.0)) _newtrack_0) (`KismetMathLibrary.VLerp` (.scale (`self.Transform_0`)) (1.0 1.0 1.0) _newtrack_0)) false false))
            (:`Finished`
              (`/Engine/EditorBlueprintResources/StandardMacros.FlipFlop`
                (:`A`
                  (if (not (`ActorComponent.IsActive` (`self.Niagara`)))
                    (`ActorComponent.Activate` (`self.Niagara`) false)
                    (`KismetSystemLibrary.Delay` 4.2)
                    (`PlayerController.ClientStartCameraShake` :`self` (`GameplayStatics.GetPlayerController` 0) :`Shake` "/Game/FX/Niagara/OrbitalBeam/beamshake.beamshake_C" :`Scale` 5.0)
                    (`KismetSystemLibrary.Delay` 5.6)
                    (goto _label_3 :!via `ReverseFromEnd`)))
                (:`B`
                  (`|ExecutionSequence`
                    (:`then_0`
                      (goto _label_2 :!via `Reset`))
                    (:`then_1`
                      (goto _label :!via `Open`))))))))))))

(fn `UserConstructionScript`
  (`parent.UserConstructionScript`))