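; Bottle actor that feeds its motion to a liquid material effect.
; Every tick it rotates itself by a fixed step, not scaled by delta time, then writes its up vector, the Bottle component's physics angular velocity and the actor's velocity into the MatC_liquid material parameter collection.
; Because the values go to a shared collection rather than a material instance, they are global to every material reading it.
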(event `self.ReceiveTick`
  (params (DeltaSeconds :type "Float (single-precision)"))
  (`self.K2_AddActorWorldRotation` (struct :`Roll` 1.0))
  (`KismetMaterialLibrary.SetVectorParameterValue` "/Game/FX/Liquid/matC_liquid.matC_liquid" "Up vector" (`KismetMathLibrary.Conv_VectorToLinearColor` (`self.GetActorUpVector`)))
  (`KismetMaterialLibrary.SetVectorParameterValue` "/Game/FX/Liquid/matC_liquid.matC_liquid" "Angular Velo" (`KismetMathLibrary.Conv_VectorToLinearColor` (`PrimitiveComponent.GetPhysicsAngularVelocityInDegrees` (`self.Bottle`) "None")))
  (`KismetMaterialLibrary.SetVectorParameterValue` "/Game/FX/Liquid/matC_liquid.matC_liquid" "Velo" (`KismetMathLibrary.Conv_VectorToLinearColor` (`self.GetVelocity`))))

(fn `UserConstructionScript`)