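; Demo Blueprint that continuously oscillates a dissolve effect through the Amount scalar of the MatC_dissolve Material Parameter Collection.
; On BeginPlay the target is set to the maximum amount, and each Tick moves the parameter toward it at a constant interpolation speed.
; When the value nearly reaches the target, a FlipFlop swaps the target between the minimum and maximum, looping the effect back and forth.
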(event `self.ReceiveBeginPlay`
  (set `self.target_amount` (`self.max_amount`)))

(event `self.ReceiveTick`
  (params (DeltaSeconds :type "Float (single-precision)"))
  (bind _returnvalue (`KismetMaterialLibrary.GetScalarParameterValue` "/Game/FX/Tuto/Dissolve/matC_dissolve.matC_dissolve" "Amount"))
  (bind _returnvalue_2 (`KismetMathLibrary.FInterpTo_Constant` _returnvalue (`self.target_amount`) DeltaSeconds 3.0))
  (`KismetMaterialLibrary.SetScalarParameterValue` "/Game/FX/Tuto/Dissolve/matC_dissolve.matC_dissolve" "Amount" _returnvalue_2)
  (if (`KismetMathLibrary.NearlyEqual_FloatFloat` _returnvalue_2 (`self.target_amount`) 1e-05)
    (`/Engine/EditorBlueprintResources/StandardMacros.FlipFlop`
      (:`A`
        (set `self.target_amount` (`self.min_ammount`)))
      (:`B`
        (set `self.target_amount` (`self.max_amount`))))))

(fn `UserConstructionScript`)