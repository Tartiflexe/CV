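; Tutorial floor spawner that builds a grid of Bp_cube actors from its own location at BeginPlay.
; A loop lays each row by chaining spawns off the previous cube's LeftLocation.
; A DoOnce captures the first cube's FrontLocation, then each following row's lead cube supplies the next front anchor.
; The Redraw event calls itself to add rows until Count exceeds Columb.
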(event `Redraw`
  (for _ (range (+ (`self.row`) 1)) :!label _label
    (bind _returnvalue (`|SpawnActorFromClass` "/Game/FX/Tuto/Floor/bp_cube.bp_cube_C" (`KismetMathLibrary.MakeTransform` (`self.next`) (struct) (`self.scale`)) "Undefined" "OverrideRootScale" null null))
    (set `self.next` (`/Game/FX/Tuto/Floor/bp_cube.left_location` _returnvalue))
    (`/Engine/EditorBlueprintResources/StandardMacros.DoOnce` false
      (:`Completed`
        (set `self.front` (`/Game/FX/Tuto/Floor/bp_cube.front_location` _returnvalue)))))
  (bind _returnvalue_2 (`|SpawnActorFromClass` "/Game/FX/Tuto/Floor/bp_cube.bp_cube_C" (`KismetMathLibrary.MakeTransform` (`self.front`) (struct) (`self.scale`)) "Undefined" "OverrideRootScale" null null))
  (set `self.next` (`/Game/FX/Tuto/Floor/bp_cube.left_location` _returnvalue_2))
  (set `self.front` (`/Game/FX/Tuto/Floor/bp_cube.front_location` _returnvalue_2))
  (if (<= (`self.count`) (`self.columb`))
    (set `self.count` (+ (`self.count`) 1))
    (`self.Redraw`)))

(event `self.ReceiveBeginPlay`
  (set `self.next` (`SceneComponent.K2_GetComponentLocation` (`self.DefaultSceneRoot`)))
  (goto _label))

(fn `UserConstructionScript`)