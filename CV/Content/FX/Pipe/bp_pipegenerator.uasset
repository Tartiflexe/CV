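; Spline-built pipe that runs a Bp_ballposition actor through itself as an effect, triggered by FxActivation or Entry1 overlap.
; The construction script lays collidable spline mesh sections and adds entry spheres at the spline ends.
; A timeline moves the spawned actor from spline start to end, then destroys it, resets MatC_pipe's Position parameter and reopens the pipe.
; Entry2 overlap does nothing, leaving the reverse direction unused.
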(event `/Game/Blueprints/cv_interface.Fx_Activation`
  (bind _spline (`self.Spline`))
  (bind _spline_2 (`self.Spline`))
  (if (`self.pipe_open?`) :!label _label
    (set `self.StartPoint` (`self.Entry2`))
    (set `self.pipe_open?` false)
    (bind _returnvalue (`|SpawnActorFromClass` "/Game/FX/Pipe/bp_ballposition.bp_ballposition_C" (`SceneComponent.K2_GetComponentToWorld` (`self.Entry2`)) "Undefined" "OverrideRootScale" null null))
    (`TimelineComponent.SetPlayRate` (`self.0-1`) (`self.Play rate`))
    (bind (_direction _length_across_spline) (`Timeline|0-1` :!via `PlayFromStart`)
      (:`Update`
        (if (== (`self.StartPoint`) (`self.Entry2`))
          (`self.K2_SetActorTransform` _returnvalue (`SplineComponent.GetTransformAtDistanceAlongSpline` _spline (`KismetMathLibrary.Lerp` 0.0 (`SplineComponent.GetSplineLength` _spline) _length_across_spline) "World" false) false false)
          (else
            (`self.K2_SetActorTransform` _returnvalue (`SplineComponent.GetTransformAtDistanceAlongSpline` _spline_2 (`KismetMathLibrary.Lerp` (`SplineComponent.GetSplineLength` _spline_2) 0.0 _length_across_spline) "World" false) false false))))
      (:`Finished`
        (`self.K2_DestroyActor` _returnvalue)
        (`KismetMaterialLibrary.SetVectorParameterValue` "/Game/FX/Pipe/matC_pipe.matC_pipe" "Position" (`KismetMathLibrary.Conv_VectorToLinearColor` (`self.maskdeformation_reset`)))
        (`self.Reset pipe entry`)))))

(event `self.Entry1.OnComponentBeginOverlap`
  (params (OverlappedComponent :type "PrimitiveComponent Object Reference") (OtherActor :type "Actor Object Reference") (OtherComp :type "PrimitiveComponent Object Reference") (OtherBodyIndex :type Integer) (bFromSweep :type Boolean) (SweepResult :type "HitResult Structure (by ref)"))
  (goto _label))

(event `Reset pipe entry`
  (set `self.pipe_open?` true))

(event `self.Entry2.OnComponentBeginOverlap`
  (params (OverlappedComponent :type "PrimitiveComponent Object Reference") (OtherActor :type "Actor Object Reference") (OtherComp :type "PrimitiveComponent Object Reference") (OtherBodyIndex :type Integer) (bFromSweep :type Boolean) (SweepResult :type "HitResult Structure (by ref)")))

(fn `UserConstructionScript`
  (bind _spline (`self.Spline`))
  (bind _spline_2 (`self.Spline`))
  (bind _sectionlenght (`self.SectionLenght`))
  (`|ExecutionSequence`
    (:`then_0`
      (bind _returnvalue (`AddComponent|NODE_AddSphereComponent-0` :`RelativeTransform` (`KismetMathLibrary.MakeTransform` (`SplineComponent.GetLocationAtSplinePoint` (`self.Spline`) 0 "Local"))))
      (`SphereComponent.SetSphereRadius` _returnvalue (`self.Approx_Size_X`) false)
      (set `self.Entry1` _returnvalue)
      (bind _returnvalue_2 (`AddComponent|NODE_AddSphereComponent-1` :`RelativeTransform` (`KismetMathLibrary.MakeTransform` (`SplineComponent.GetLocationAtSplinePoint` (`self.Spline`) (`SplineComponent.GetNumberOfSplinePoints` (`self.Spline`)) "Local"))))
      (`SphereComponent.SetSphereRadius` _returnvalue_2 (`self.Approx_Size_X`) false)
      (set `self.Entry2` _returnvalue_2))
    (:`then_1`
      (for _index (range (+ (`KismetMathLibrary.FTrunc` (/ (`SplineComponent.GetSplineLength` (`self.Spline`)) (`self.SectionLenght`))) 1))
        (bind _returnvalue_3 (`AddComponent|NODE_AddSplineMeshComponent-1`))
        (`PrimitiveComponent.SetCollisionEnabled` _returnvalue_3 "QueryAndPhysics")
        (`SplineMeshComponent.SetForwardAxis` _returnvalue_3 "Z" true)
        (bind _returnvalue_4 (* _index _sectionlenght))
        (bind _returnvalue_5 (* (+ _index 1) _sectionlenght))
        (`SplineMeshComponent.SetStartAndEnd` _returnvalue_3 (`SplineComponent.GetLocationAtDistanceAlongSpline` _spline_2 _returnvalue_4 "Local") (`KismetMathLibrary.ClampVectorSize` (`SplineComponent.GetTangentAtDistanceAlongSpline` _spline_2 _returnvalue_4 "Local") 0.0 (`self.SectionLenght`)) (`SplineComponent.GetLocationAtDistanceAlongSpline` _spline _returnvalue_5 "Local") (`KismetMathLibrary.ClampVectorSize` (`SplineComponent.GetTangentAtDistanceAlongSpline` _spline _returnvalue_5 "Local") 0.0 (`self.SectionLenght`)) true)
        (`PrimitiveComponent.SetCollisionObjectType` _returnvalue_3 "ECC_GameTraceChannel2")
        (set `ActorComponent.ComponentTags` (`self.Taglist`) _returnvalue_3)))))