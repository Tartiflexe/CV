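; Orbital beam cannon Blueprint that plays a firing effect with spinning rings when the Fire input is pressed.
; A timeline curve, scaled by differing speeds and directions, sets the yaw step that Tick applies to the top, middle and bottom ring meshes.
; The same press activates the Niagara beam effect, then plays a camera shake on the first player controller after a fixed delay.
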(event `self.ReceiveTick`
  (params (DeltaSeconds :type "Float (single-precision)"))
  (`|ExecutionSequence`
    (:`then_0`
      (`SceneComponent.K2_AddLocalRotation` (`self.Msh_OrbitalCanon_Msh_TopRing`) (`KismetMathLibrary.MakeRotator` 0.0 0.0 (`self.Rot_TopRing`)) false false))
    (:`then_1`
      (`SceneComponent.K2_AddLocalRotation` (`self.Msh_OrbitalCanon_Msh_MdlRing`) (`KismetMathLibrary.MakeRotator` 0.0 0.0 (`self.Rot_MdlRing`)) false false))
    (:`then_2`
      (`SceneComponent.K2_AddLocalRotation` (`self.Msh_OrbitalCanon_Msh_BtmRing`) (`KismetMathLibrary.MakeRotator` 0.0 0.0 (`self.Rot_BtmRing`)) false false))))

(event `InputAction|Fire`
  (params (Key :type "Key Structure"))
  (:`Pressed`
    (`|ExecutionSequence`
      (:`then_0`
        (set `self.Speed_TopRing` 0.55)
        (set `self.Speed_MdlRing` -0.4)
        (set `self.Speed_BtmRing` 0.3)
        (bind (_direction _crv_cannonrot) (`Timeline|Timeline_0`)
          (:`Update`
            (set `self.Rot_TopRing` (* _crv_cannonrot (`self.Speed_TopRing`)))
            (set `self.Rot_MdlRing` (* _crv_cannonrot (`self.Speed_MdlRing`)))
            (set `self.Rot_BtmRing` (* _crv_cannonrot (`self.Speed_BtmRing`))))))
      (:`then_1`
        (`ActorComponent.Activate` (`self.Niagara`) false)
        (`KismetSystemLibrary.Delay` 4.2)
        (`PlayerController.ClientStartCameraShake` :`self` (`GameplayStatics.GetPlayerController` 0) :`Shake` "/Game/FX/Niagara/OrbitalBeam/beamshake.beamshake_C" :`Scale` 5.0)))))

(fn `UserConstructionScript`)